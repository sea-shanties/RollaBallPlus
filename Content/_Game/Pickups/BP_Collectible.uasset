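; BP_Collectible is a pickup that the player collects by touching it.
; When its Box begins overlapping player 0's pawn, it increments CollectibleCount on that player's BallPlayerState.
; It then plays a coin sound and spawns a burst effect at its location before destroying itself.
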(event OnComponentBeginOverlap(Box)
  (params (OverlappedComponent :type Primitive%20Component%20Object%20Reference) (OtherActor :type Actor%20Object%20Reference) (OtherComp :type Primitive%20Component%20Object%20Reference) (OtherBodyIndex :type Integer) (bFromSweep :type Boolean) (SweepResult :type Hit%20Result%20Structure%20%28by%20ref%29))
  (bind _returnvalue (Transformation|GetActorLocation))
  (if (== OtherActor (Game|Player|GetPlayerPawn 0))
    (bind _asball_player_state (Utilities|Casting|CastToBallPlayerState (Game|GetPlayerState 0)))
    (Variables|/Game/_Game/BallGame/BallPlayerState.BallPlayerState_C|SetCollectibleCount _asball_player_state (+ (Variables|/Game/_Game/BallGame/BallPlayerState.BallPlayerState_C|GetCollectibleCount _asball_player_state) 1))
    (Audio|PlaySoundatLocation "/Game/_Game/Audio/coinPickup_Cue.coinPickup_Cue" _returnvalue "0, 0, 0" 1.0 1.0 0.0 0 0 0 0)
    (Niagara|SpawnSystematLocation "/Game/_Game/Particles/PS_GenericBurst.PS_GenericBurst" _returnvalue)
    (Actor|DestroyActor)))

(fn ConstructionScript)